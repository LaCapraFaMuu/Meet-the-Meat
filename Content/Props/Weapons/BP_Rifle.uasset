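; Rifle weapon actor whose Fire event shoots a damaging projectile with muzzle flash and sound.
; Fire spawns a non-uniformly scaled BP_Projectile at the ProjectileSpawnPosition component's transform and copies the rifle's Damage value onto it.
; It then attaches a scaled-down muzzle flash emitter at the root component's muzzle socket and plays the fire sound at the actor's location.
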(event EventBeginPlay
  (|CallParentFunction) ; This node is disabled and will not be called.\nDrag off pins to build functionality.
)

(event Collision|EventActorBeginOverlap
  (params (OtherActor :type Actor%20Object%20Reference))
  (|CallParentFunction OtherActor) ; This node is disabled and will not be called.\nDrag off pins to build functionality.
)

(event EventTick
  (params (DeltaSeconds :type Float%20%28single-precision%29))
  (|CallParentFunction DeltaSeconds) ; This node is disabled and will not be called.\nDrag off pins to build functionality.
)

(event EventFire
  (bind _projectile_spawn_position (Variables|Default|GetProjectile%20Spawn%20Position))
  (bind _rootcomponent (Variables|Transformation|GetRootComponent))
  (bind _returnvalue (Transformation|GetSocketTransform _rootcomponent "muzzle" "RTS_World"))
  (bind _returnvalue_2 (Transformation|GetWorldTransform _projectile_spawn_position))
  (bind _returnvalue_3 (Game|SpawnActorfromClass "/Game/Props/Weapons/BP_Projectile.BP_Projectile_C" (Math|Transform|MakeTransform (.location _returnvalue_2) (.rotation _returnvalue_2) "0.600000,0.200000,0.200000") "Undefined" "MultiplyWithRoot" 0 0))
  (Variables|/Game/Props/Weapons/BP_Projectile.BP_Projectile_C|SetDamage _returnvalue_3 (Variables|Default|GetDamage))
  (Effects|SpawnEmitterAttached "/Game/InfinityBladeEffects/Effects/FX_Monsters/FX_Monster_Gruntling/Master/P_BackPack_MuzzleFlash.P_BackPack_MuzzleFlash" _rootcomponent "muzzle" (.location _returnvalue) (.rotation _returnvalue) "0.050000,0.050000,0.050000" "KeepWorldPosition" true "AutoRelease")
  (Audio|PlaySoundatLocation "/Game/Audios/MS_Fire.MS_Fire" (Transformation|GetActorLocation) "0, 0, 0" 1.0 1.0 0.0 0 0 0 0))

(fn ConstructionScript
  (|CallParentFunction))