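; BP_Projectile is a weapon projectile actor that damages what it hits.
; A hit on the Bullet component spawns a scaled-down impact particle aligned to the surface normal, applies Damage to the hit actor, and destroys the projectile if that actor is valid.
; ProjectileMovement bounce events increment a counter that also destroys the projectile once it exceeds a small fixed limit.
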(event OnProjectileBounce(ProjectileMovement)
  (params (ImpactResult :type Hit%20Result%20Structure%20%28by%20ref%29) (ImpactVelocity :type Vector%20%28by%20ref%29 :default "0, 0, 0"))
  (bind _output_get (Variables|Default|SetBounceNumber (+ (Variables|Default|GetBounceNumber) 1)))
  (if (> _output_get 2)
    (Actor|DestroyActor)))

(event OnComponentHit(Bullet)
  (params (HitComponent :type Primitive%20Component%20Object%20Reference) (OtherActor :type Actor%20Object%20Reference) (OtherComp :type Primitive%20Component%20Object%20Reference) (NormalImpulse :type Vector :default "0, 0, 0") (Hit :type Hit%20Result%20Structure%20%28by%20ref%29))
  (bind (_bblockinghit _binitialoverlap _time _distance _location _impactpoint _normal _impactnormal _physmat _hitactor) (Collision|BreakHitResult Hit))
  (Effects|SpawnEmitteratLocation "/Game/Effects/ShootingEffects/FX_Monsters/FX_Monster_Troll/death/P_TrollDeathImpact.P_TrollDeathImpact" _impactpoint (Math|Rotator|MakeRotfromX _normal) "0.500000,0.500000,0.500000")
  (Game|Damage|ApplyDamage _hitactor (Variables|Default|GetDamage) 0 0)
  (Utilities|IsValid _hitactor
    (:Is%20Valid
      (Actor|DestroyActor))))

(event EventBeginPlay)

(event Collision|EventActorBeginOverlap
  (params (OtherActor :type Actor%20Object%20Reference)))

(event EventTick
  (params (DeltaSeconds :type Float%20%28single-precision%29)))

(fn ConstructionScript)