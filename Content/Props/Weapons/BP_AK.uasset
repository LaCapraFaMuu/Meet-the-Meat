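; BP_AK is a hitscan rifle actor whose Fire event shoots from the muzzle socket on its root component.
; It line-traces forward on the Visibility channel with debug drawing on, and on a hit spawns a scaled-down impact particle and applies fixed damage to the hit actor.
; Every shot also spawns an attached muzzle flash at the socket and plays a fire sound, whether or not it hits.
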(event EventBeginPlay
  (|CallParentFunction) ; This node is disabled and will not be called.\nDrag off pins to build functionality.
)

(event Collision|EventActorBeginOverlap
  (params (OtherActor :type Actor%20Object%20Reference))
  (|CallParentFunction OtherActor) ; This node is disabled and will not be called.\nDrag off pins to build functionality.
)

(event EventTick
  (params (DeltaSeconds :type Float%20%28single-precision%29))
  (|CallParentFunction DeltaSeconds) ; This node is disabled and will not be called.\nDrag off pins to build functionality.
)

(event EventFire
  (bind _rootcomponent (Variables|Transformation|GetRootComponent))
  (bind _rootcomponent_2 (Variables|Transformation|GetRootComponent))
  (bind _returnvalue (Transformation|GetSocketTransform _rootcomponent_2 "muzzle" "RTS_World"))
  (bind _returnvalue_2 (Transformation|GetSocketTransform _rootcomponent "muzzle" "RTS_World"))
  (Utilities|FlowControl|Sequence
    (:then_0
      (bind (_outhit _returnvalue_3) (Collision|LineTraceByChannel (.location _returnvalue_2) (+ (.location _returnvalue_2) (* (Math|Vector|GetForwardVector (.rotation _returnvalue_2)) 5e+03)) "TraceTypeQuery1" false 0 "ForDuration"))
      (if _returnvalue_3
        (Effects|SpawnEmitteratLocation "/Game/Effects/ShootingEffects/FX_Monsters/FX_Monster_Troll/death/P_TrollDeathImpact.P_TrollDeathImpact" (.ImpactPoint (Collision|BreakHitResult _outhit)) (Math|Rotator|MakeRotfromX (.Normal (Collision|BreakHitResult _outhit))) "0.500000,0.500000,0.500000")
        (Game|Damage|ApplyDamage (.HitActor (Collision|BreakHitResult _outhit)) 15.0 0 0)))
    (:then_1
      (Effects|SpawnEmitterAttached "/Game/Effects/ShootingEffects/FX_Monsters/FX_Monster_Gruntling/Master/P_BackPack_MuzzleFlash.P_BackPack_MuzzleFlash" _rootcomponent_2 "muzzle" (.location _returnvalue) (.rotation _returnvalue) "0.050000,0.050000,0.050000" "KeepWorldPosition" true "AutoRelease")
      (Audio|PlaySoundatLocation "/Game/Audios/MS_Fire.MS_Fire" (Transformation|GetActorLocation) "0, 0, 0" 1.0 1.0 0.0 0 0 0 0))))

(fn ConstructionScript
  (|CallParentFunction))