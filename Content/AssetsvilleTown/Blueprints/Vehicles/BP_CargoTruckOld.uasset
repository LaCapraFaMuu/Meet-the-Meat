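; BP_CargoTruckOld is a drivable cargo truck that the player character can possess and exit.
; Tick feeds throttle, brake, steering and handbrake input to the vehicle movement component, while Enhanced Input handles look and a first/third-person camera toggle.
; Entering hides the character, shows a driver stand-in and stores two capsule references.
; Pressing E repossesses the character at an exit point and restores visibility and capsule collision.
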(event Input|EnhancedActionEvents|EnhancedInputActionIA_SwitchCamera
  (params (ActionValue :type Boolean) (ElapsedSeconds :type Float%20%28double-precision%29) (TriggeredSeconds :type Float%20%28double-precision%29) (InputAction :type Input%20Action%20Object%20Reference :default "/Game/Player/Input/Actions/IA_SwitchCamera.IA_SwitchCamera"))
  ;[1 1 1] Switch Camera
  (:Started
    (Utilities|FlowControl|FlipFlop
      (:A
        (Components|Activation|SetActive (Variables|Default|GetThirdPersonCamera) true false)
        (Components|Activation|SetActive (Variables|Default|GetFirstPersonCamera) false false)
        (Variables|Default|SetbUseControllerRotationYaw false))
      (:B
        (Components|Activation|SetActive (Variables|Default|GetThirdPersonCamera) false false)
        (Components|Activation|SetActive (Variables|Default|GetFirstPersonCamera) true false)
        (Variables|Default|SetbUseControllerRotationYaw true)))))

(event Input|EnhancedActionEvents|EnhancedInputActionIA_Look
  (params (ActionValue :type Vector%202D%20Structure) (ElapsedSeconds :type Float%20%28double-precision%29) (TriggeredSeconds :type Float%20%28double-precision%29) (InputAction :type Input%20Action%20Object%20Reference :default "/Game/Player/Input/Actions/IA_Look.IA_Look"))
  ;[1 1 1] Camera Movment
  (Pawn|Input|AddControllerYawInput (.x ActionValue))
  (Pawn|Input|AddControllerPitchInput (.y ActionValue)))

(event EventEnterVehicle
  (params (Player%20Character :type Pawn%20Object%20Reference) (CapsuleCollision :type Capsule%20Component%20Object%20Reference) (CapsuleCollision2 :type Capsule%20Component%20Object%20Reference))
  ;[1 1 1] Enter Vehicle
  (Pawn|Possess (Game|GetPlayerController 0) self)
  (Variables|Default|SetPlayer%20Character Player%20Character)
  (Rendering|SetActorHiddenInGame (Variables|Default|GetPlayer%20Character) true)
  (Development|SetHiddeninGame (Variables|Default|GetPlayer%20Driving) false false)
  (Variables|Default|SetCapsule%20Collision CapsuleCollision)
  (Variables|Default|SetCapsule%20Collision%202 CapsuleCollision2))

(event EventTick
  (params (DeltaSeconds :type Float%20%28single-precision%29))
  (bind _vehiclemovementcomponent (Variables|Default|GetVehicleMovementComponent))
  ;[1 1 1] Driving
  (Class|ChaosVehicleMovementComponent|SetThrottleInput _vehiclemovementcomponent (Input|AxisValues|GetThrottle_Input))
  (Class|ChaosVehicleMovementComponent|SetBrakeInput _vehiclemovementcomponent (Input|AxisValues|GetBrake_Input))
  (Class|ChaosVehicleMovementComponent|SetSteeringInput _vehiclemovementcomponent (Input|AxisValues|GetSteering_Input))
  (Class|ChaosVehicleMovementComponent|SetHandbrakeInput _vehiclemovementcomponent (== (Input|AxisValues|GetHandbrake_Input) 1.0))
  (Transformation|AddRelativeRotation (Variables|Default|GetSpringArm) "0, 0, 0" false false))

(event Input|KeyboardEvents|E
  (params (Key :type Key%20Structure :default "None"))
  ;[1 1 1] Exit Vehicle
  (:Pressed
    (Pawn|Possess (Game|GetPlayerController 0) (Variables|Default|GetPlayer%20Character))
    (Transformation|SetActorLocationAndRotation (Variables|Default|GetPlayer%20Character) (.location (Transformation|GetWorldTransform (Variables|Default|GetPlayer%20Character%20Exit%20REF))) "0, 0, 0" false true)
    (Rendering|SetActorHiddenInGame (Variables|Default|GetPlayer%20Character) false)
    (Development|SetHiddeninGame (Variables|Default|GetPlayer%20Driving) true false)
    (Collision|SetCollisionEnabled (Variables|Default|GetCapsule%20Collision) "QueryAndPhysics")
    (Collision|SetCollisionEnabled (Variables|Default|GetCapsule%20Collision%202) "QueryAndPhysics")
    (Variables|/Script/Engine.PlayerCameraManager|SetViewPitchMax (Game|GetPlayerCameraManager 0) 1e+02)))

(fn ConstructionScript)