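; BP_CivilianAIFemale3 is a female civilian AI NPC Blueprint that handles taking damage and death.
; AnyDamage forwards the damage through MultiAnyDamage to the BPCStats component's DecreaseHealth.
; When that returns true, the mesh simulates physics as a ragdoll, then after a short delay is hidden and the capsule's collision is disabled, without destroying the actor.
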(event Custom|MultiAnyDamage
  (params (Target :type BPC%20Stats%20Object%20Reference) (Damage :type Float%20%28double-precision%29))
  (bind _isdead (Default|DecreaseHealth Target Damage))
  (if _isdead
    (Physics|SetSimulatePhysics (Variables|Character|GetMesh) true)
    (Utilities|FlowControl|Delay 3.0)
    (Rendering|SetVisibility (Variables|Character|GetMesh) false false)
    (Collision|SetCollisionEnabled (Variables|Collision|GetCapsuleComponent) "NoCollision")))

(event Game|Damage|EventAnyDamage
  (params (Damage :type Float%20%28single-precision%29) (DamageType :type Damage%20Type%20Object%20Reference) (InstigatedBy :type Controller%20Object%20Reference) (DamageCauser :type Actor%20Object%20Reference))
  (CallFunction|MultiAnyDamage (Variables|Default|GetBPC_Stats) Damage))

(fn ConstructionScript)