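; BPC_Stats is a player stats component that tracks current health against a maximum.
; Current health starts at the maximum on BeginPlay.
; DecreaseHealth subtracts damage without clamping and returns whether health has reached zero or below, while IncreaseHealth adds health and caps it at the maximum.
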(event EventBeginPlay
  (Variables|Health|SetCurrentHealth (Variables|Health|GetMaxHealth)))

(fn DecreaseHealth
  (params (Damage :type Float%20%28double-precision%29))
  (Variables|Health|SetCurrentHealth (- (Variables|Health|GetCurrentHealth) Damage))
  (if (<= (Variables|Health|GetCurrentHealth) 0.0)
    (return true)
    (else
      (return false))))

(fn IncreaseHealth
  (params (AddedHealth :type Float%20%28double-precision%29))
  (Variables|Health|SetCurrentHealth (+ (Variables|Health|GetCurrentHealth) AddedHealth))
  (if (> (Variables|Health|GetCurrentHealth) (Variables|Health|GetMaxHealth))
    (Variables|Health|SetCurrentHealth (Variables|Health|GetMaxHealth))))